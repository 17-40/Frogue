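; BP_Legless is an enemy bug that patrols between its position and random nearby points, then attacks the player.
; Pawn sensing or taking damage makes it move to the target and launch impulse-driven projectiles at close range on a cooldown.
; Box overlaps and explosion events reduce health, driving an animated lifebar, damage numbers and death effects.
; A sphere toggles lifebar visibility and, on exit, resumes patrol after a delay.
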(event OnComponentBeginOverlap(Sphere)
  (params (OverlappedComponent :type Primitive%20Component%20Object%20Reference) (OtherActor :type Actor%20Object%20Reference) (OtherComp :type Primitive%20Component%20Object%20Reference) (OtherBodyIndex :type Integer) (bFromSweep :type Boolean) (SweepResult :type Hit%20Result%20Structure%20%28by%20ref%29))
  ;[1 1 1] Убирает/показывает
  (Utilities|Casting|CastTo OtherActor)
  (Rendering|SetVisibility (Variables|Default|GetLifebar) true false))

(event OnComponentEndOverlap(Sphere)
  (params (OverlappedComponent :type Primitive%20Component%20Object%20Reference) (OtherActor :type Actor%20Object%20Reference) (OtherComp :type Primitive%20Component%20Object%20Reference) (OtherBodyIndex :type Integer))
  ;[1 1 1] Убирает/показывает
  (Utilities|Casting|CastTo OtherActor)
  (Rendering|SetVisibility (Variables|Default|GetLifebar) false false)
  ;[1 1 1] Теряет
  (Utilities|FlowControl|RetriggerableDelay 2.0)
  (Variables|Default|SetSeeEnemy false)
  (Utilities|FlowControl|RetriggerableDelay 0.25)
  (if (not (Variables|Default|GetSeeEnemy))
    (CallFunction|Patrol)))

(event OnSeePawn(PawnSensing)
  (params (Pawn :type Pawn%20Object%20Reference))
  (bind _returnvalue (Transformation|GetActorLocation))
  (bind _asfirst_person_character (Utilities|Casting|CastTo Pawn))
  (Utilities|FlowControl|Sequence
    (:then_0
      (if (not (Variables|Default|GetSeeEnemy))
        (Audio|SpawnSoundatLocation 0 (Transformation|GetActorLocation) "0, 0, 0" 1.0 1.0 0.0 0 0)))
    (:then_1
      (Variables|Default|SetSeeEnemy true)
      (AI|AIMoveTo self (Transformation|GetActorLocation _asfirst_person_character) 0 1e+01 false
        (:then
          (Utilities|FlowControl|Sequence
            (:then_0
              ;[1 1 1] Поворачивается к персонажу
              (Transformation|SetActorRotation (Math|Rotator|MakeRotator (.roll (Math|Rotator|FindLookatRotation _returnvalue (Transformation|GetActorLocation _asfirst_person_character))) 0.0 (.yaw (Math|Rotator|FindLookatRotation _returnvalue (Transformation|GetActorLocation _asfirst_person_character))))))
            (:then_1
              (if (< (Math|Vector|Distance(Vector) _returnvalue (Transformation|GetActorLocation _asfirst_person_character)) 2e+02)
                ;[1 1 1] Стреляет в персонажа
                (if (Variables|Default|GetSpawnProjectile)
                  (Variables|Default|SetBug1State 0)
                  (bind _returnvalue_2 (Game|SpawnActorfromClass 0 (Transformation|GetWorldTransform (Variables|Default|GetScene)) "Undefined" 0 0))
                  (Development|PrintString "Hello")
                  (Audio|SpawnSoundatLocation 0 (Transformation|GetActorLocation) "0, 0, 0" 1.0 1.0 0.0 0 0)
                  (Physics|AddImpulse (Variables|Default|GetCollisionComponent _returnvalue_2) (* (Math|Vector|GetForwardVector (Variables|Character|GetMesh)) (Variables|Default|GetShootAmount)) "None" true)
                  (Variables|Default|SetSpawnProjectile false)
                  (Utilities|FlowControl|Delay 1.5)
                  (Variables|Default|SetSpawnProjectile true)
                  (if (Variables|Default|GetHURT)
                    (Variables|Default|SetBug1State 0)
                    (else
                      (Variables|Default|SetBug1State 0))))))))
        (:OnFail
          (Utilities|FlowControl|Delay 0.2)
          (AI|AIMoveTo 0 (Transformation|GetActorLocation) 0 5.0 false))))))

(event OnComponentBeginOverlap(Box)
  (params (OverlappedComponent :type Primitive%20Component%20Object%20Reference) (OtherActor :type Actor%20Object%20Reference) (OtherComp :type Primitive%20Component%20Object%20Reference) (OtherBodyIndex :type Integer) (bFromSweep :type Boolean) (SweepResult :type Hit%20Result%20Structure%20%28by%20ref%29))
  (bind _returnvalue (Transformation|GetActorLocation))
  (bind _charactermovement (Variables|Character|GetCharacterMovement))
  (Utilities|Casting|CastTo OtherActor
    (:then
      _)
    (:CastFailed
      (Utilities|Casting|CastTo OtherActor)))
  (if (not (Variables|Default|GetOn))
    (Variables|Default|SetOn true)
    (Class|Object|ManafromEnemy(Message) (Game|GetPlayerCharacter 0))
    ;[1 1 1] Урон
    (Variables|Default|SetBug%201%20health (- (Variables|Default|GetBug%201%20health) (Variables|Default|GetDamage (.Char%20ref (Variables|Default|GetChar%20ref)))))
    (Audio|SpawnSoundatLocation 0 (Transformation|GetActorLocation) "0, 0, 0" 1.0 1.0 0.0 0 0)
    (Variables|Default|SetHURT true)
    (Variables|Default|SetBug1State 0)
    (CallFunction|TRIGGER)
    (Utilities|FlowControl|Sequence
      (:then_0
        ;[1 1 1] Лайфбар
        (Variables|Default|Sethealth (.Lifebar%20Ref (Variables|Default|GetLifebar%20Ref)) (Variables|Default|GetBug%201%20health))
        (Class|Object|CombatNumbers(Message) (UserInterface|GetWidget (Variables|Default|GetDamageNumber)))
        (CallFunction|Lifebaranim)
        (Variables|Default|SetOn false)
        ;[1 1 1] Смерть
        (if (<= (Variables|Default|GetBug%201%20health) 0.0)
          (Niagara|SpawnSystematLocation 0 _returnvalue "0, 0, 0" "0.200000,0.200000,0.200000")
          (Rendering|SetVisibility (Variables|Default|GetLifebar) false false)
          (Actor|DestroyActor)
          (else
            (Niagara|SpawnSystematLocation 0 _returnvalue "0, 0, 0" "0.200000,0.200000,0.200000"))))
      (:then_1
        (if (Utilities|IsValid _charactermovement)
          (Variables|/Script/Engine.CharacterMovementComponent|SetMaxWalkSpeed _charactermovement 4e+02)
          (Utilities|FlowControl|Delay 0.2)
          (Variables|Default|SetBug1State 0))))))

(event Custom|lifebaranim
  (bind _newtrack_3 (Timeline|Timeline_0 PlayFromStart)
    (:Update
      (Transformation|SetRelativeScale3D (Variables|Default|GetLifebar) _newtrack_3))
    (:Finished
      (bind _newtrack_3_2 (Timeline|Timeline_1 ReverseFromEnd)
        (:Update
          (Transformation|SetRelativeScale3D (Variables|Default|GetLifebar) _newtrack_3_2))))))

(event Custom|New%20Locations
  (bind _returnvalue (Transformation|GetActorLocation))
  ;[1 1 1] Локации для перемещения
  (Variables|Patrol|SetLocation1 _returnvalue)
  (Variables|Patrol|SetLocation2 (+ _returnvalue (Math|Vector|MakeVector (Math|Conversions|ToFloat(Integer) (Math|Random|RandomIntegerinRange -2000 2000)) (Math|Conversions|ToFloat(Integer) (Math|Random|RandomIntegerinRange -2000 2000)) 0.0)))
  (CallFunction|Patrol))

(event Custom|TRIGGER
  (bind _returnvalue (Transformation|GetActorLocation))
  (bind _asfirst_person_character (Utilities|Casting|CastTo (stale OnSeePawn(PawnSensing) Pawn)))
  (Utilities|FlowControl|Sequence
    (:then_0
      (if (not (Variables|Default|GetSeeEnemy))
        (Audio|SpawnSoundatLocation 0 (Transformation|GetActorLocation) "0, 0, 0" 1.0 1.0 0.0 0 0)))
    (:then_1
      (Variables|Default|SetSeeEnemy true)
      (AI|AIMoveTo self (Transformation|GetActorLocation _asfirst_person_character) 0 1e+01 false
        (:then
          (Utilities|FlowControl|Sequence
            (:then_0
              ;[1 1 1] Поворачивается к персонажу
              (Transformation|SetActorRotation (Math|Rotator|MakeRotator (.roll (Math|Rotator|FindLookatRotation _returnvalue (Transformation|GetActorLocation _asfirst_person_character))) 0.0 (.yaw (Math|Rotator|FindLookatRotation _returnvalue (Transformation|GetActorLocation _asfirst_person_character))))))
            (:then_1
              (if (< (Math|Vector|Distance(Vector) _returnvalue (Transformation|GetActorLocation _asfirst_person_character)) 2e+02)
                ;[1 1 1] Стреляет в персонажа
                (if (Variables|Default|GetSpawnProjectile)
                  (Variables|Default|SetBug1State 0)
                  (bind _returnvalue_2 (Game|SpawnActorfromClass 0 (Transformation|GetWorldTransform (Variables|Default|GetScene)) "Undefined" 0 0))
                  (Development|PrintString "Hello")
                  (Audio|SpawnSoundatLocation 0 (Transformation|GetActorLocation) "0, 0, 0" 1.0 1.0 0.0 0 0)
                  (Physics|AddImpulse (Variables|Default|GetCollisionComponent _returnvalue_2) (* (Math|Vector|GetForwardVector (Variables|Character|GetMesh)) (Variables|Default|GetShootAmount)) "None" true)
                  (Variables|Default|SetSpawnProjectile false)
                  (Utilities|FlowControl|Delay 1.5)
                  (Variables|Default|SetSpawnProjectile true)
                  (if (Variables|Default|GetHURT)
                    (Variables|Default|SetBug1State 0)
                    (else
                      (Variables|Default|SetBug1State 0))))))))
        (:OnFail
          (Utilities|FlowControl|Delay 0.2)
          (AI|AIMoveTo 0 (Transformation|GetActorLocation) 0 5.0 false))))))

(event Custom|Patrol
  (bind _self self)
  (if (Variables|Default|GetPatrol%20Loc%201)
    (Utilities|PatrolLocations true false
      (:Out
        (AI|AIMoveTo _self (Variables|Patrol|GetLocation1) 0 5.0 false
          (:OnSuccess
            (Utilities|PatrolLocations false true :!label _label
              (:Out
                (AI|AIMoveTo _self (Variables|Patrol|GetLocation2) 0 5.0 false
                  (:OnSuccess
                    (Utilities|PatrolLocations true false
                      (:Out
                        (CallFunction|NewLocations))))
                  (:OnFail
                    (CallFunction|NewLocations))))))
          (:OnFail
            (CallFunction|NewLocations)))))
    (elif (Variables|Default|GetPatrol%20Loc%202)
      (goto _label))))

(event EventBeginPlay
  (bind _returnvalue (Transformation|GetActorLocation))
  (Utilities|FlowControl|Sequence
    (:then_0
      ;[1 1 1] Референсы
      (bind _asfirst_person_character (Utilities|Casting|CastTo (Game|GetPlayerCharacter 0)))
      (Variables|Default|SetChar%20Ref 0 _asfirst_person_character)
      (bind _asenemy_lifebar (Utilities|Casting|CastTo (UserInterface|GetUserWidgetObject (Variables|Default|GetLifebar))))
      (Variables|Default|SetLifebar%20Ref 0 _asenemy_lifebar)
      (Variables|Default|SetMaxHealth (.Lifebar%20Ref (Variables|Default|GetLifebar%20Ref)) (Variables|Default|GetBug%201%20health)))
    (:then_1
      ;[1 1 1] Локации для перемещения
      (Variables|Patrol|SetLocation1 _returnvalue)
      (Variables|Patrol|SetLocation2 (+ _returnvalue (Math|Vector|MakeVector (Math|Conversions|ToFloat(Integer) (Math|Random|RandomIntegerinRange -2000 2000)) (Math|Conversions|ToFloat(Integer) (Math|Random|RandomIntegerinRange -2000 2000)) 0.0)))
      (CallFunction|Patrol))))

(event EventRadialBOOM
  (bind _returnvalue (Transformation|GetActorLocation))
  ;[1 1 1] Урон от бочки или гранаты
  (bind _output_get (Variables|Default|SetBug%201%20health (- (Variables|Default|GetBug%201%20health) 7e+01)))
  ;[1 1 1] Лайфбар
  (Variables|Default|Sethealth (.Lifebar%20Ref (Variables|Default|GetLifebar%20Ref)) _output_get)
  (Class|Object|CombatNumbers(Message) (UserInterface|GetWidget (Variables|Default|GetDamageNumber)))
  (CallFunction|Lifebaranim)
  (Variables|Default|SetOn false)
  ;[1 1 1] Смерть
  (if (<= (Variables|Default|GetBug%201%20health) 0.0)
    (Niagara|SpawnSystematLocation 0 _returnvalue "0, 0, 0" "0.200000,0.200000,0.200000")
    (Rendering|SetVisibility (Variables|Default|GetLifebar) false false)
    (Actor|DestroyActor)
    (else
      (Niagara|SpawnSystematLocation 0 _returnvalue "0, 0, 0" "0.200000,0.200000,0.200000"))))

(event EventTick
  (params (DeltaSeconds :type Float%20%28single-precision%29))
  ;[1 1 1] Если между актерами нет препятствий, то агрится
)

(event EventBUGBOOM
  (bind _returnvalue (Transformation|GetActorLocation))
  ;[1 1 1] Урон от бочки или гранаты
  (bind _output_get (Variables|Default|SetBug%201%20health (- (Variables|Default|GetBug%201%20health) 7e+01)))
  ;[1 1 1] Лайфбар
  (Variables|Default|Sethealth (.Lifebar%20Ref (Variables|Default|GetLifebar%20Ref)) _output_get)
  (Class|Object|CombatNumbers(Message) (UserInterface|GetWidget (Variables|Default|GetDamageNumber)))
  (CallFunction|Lifebaranim)
  (Variables|Default|SetOn false)
  ;[1 1 1] Смерть
  (if (<= (Variables|Default|GetBug%201%20health) 0.0)
    (Niagara|SpawnSystematLocation 0 _returnvalue "0, 0, 0" "0.200000,0.200000,0.200000")
    (Rendering|SetVisibility (Variables|Default|GetLifebar) false false)
    (Actor|DestroyActor)
    (else
      (Niagara|SpawnSystematLocation 0 _returnvalue "0, 0, 0" "0.200000,0.200000,0.200000"))))

(event EventDestroyed
  (Audio|SpawnSoundatLocation 0 (Transformation|GetActorLocation) "0, 0, 0" 1.0 1.0 0.0 0 0))

(fn ConstructionScript)

(fn GetRandomLocation
  (Variables|Default|SetCurrentPatrolpoints (Math|Random|RandomInteger (Utilities|Array|Length (Variables|Default|GetPatrolPoints)))))